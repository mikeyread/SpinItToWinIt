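; BPC_Debug is a debug component that spawns visual helper actors for spheres and trace hits at runtime.
; Sphere requests are grouped by key in an actor map, reusing that key's BP_DebugSphere or spawning and registering one.
; When a sphere actor signals it has no active spheres, the component unregisters and destroys it.
; Each hit trace request spawns a separate BP_HitDebug with a timed lifespan.
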(event Custom|SpawnDebugSphere
  (params (DebugKey :type Name) (SphereColour :type Linear%20Color%20Structure :default "(R=2.000000,G=0.637436,B=0.002299,A=1.000000)") (LineWidth :type Float%20%28single-precision%29) (Sphere%20Location :type Vector) (SpereSize :type Vector :default "0.500000,0.500000,0.500000") (World%20Space :type Boolean) (MaxDebugSpheres :type Integer) (DebugLifetime :type Float%20%28single-precision%29))
  (bind _debugactormap (Variables|Default|GetDebugActorMap))
  (bind _output_get (Variables|Default|SetDebug%20Key DebugKey))
  (if (Utilities|Map|Contains _debugactormap _output_get)
    (Default|SpawnDebugSpere (.Value (Utilities|Map|Find _debugactormap _output_get)) SphereColour LineWidth Sphere%20Location SpereSize World%20Space MaxDebugSpheres DebugLifetime)
    (else
      (bind _returnvalue (Game|SpawnActorfromClass "/Game/Blueprints/Debug/BP_DebugSphere.BP_DebugSphere_C" (Transformation|GetActorTransform (Components|GetOwner)) "Undefined" "MultiplyWithRoot" 0 SphereColour LineWidth Sphere%20Location SpereSize World%20Space MaxDebugSpheres DebugLifetime 0))
      (Utilities|Map|Add (Variables|Default|GetDebugActorMap) (Variables|Default|GetDebug%20Key) _returnvalue)
      (EventDispatchers|BindEventtoNoActiveSpheres _returnvalue (delegate Custom|DestroyDebugActor)))))

(event Custom|DestroyDebugActor
  (params (Actor :type BP%20Debug%20Sphere%20Object%20Reference))
  (bind _debugactormap (Variables|Default|GetDebugActorMap))
  (bind _values (Utilities|Map|Values (Variables|Default|GetDebugActorMap)))
  (bind (_array_element _array_index) (Utilities|Array|ForEachLoopwithBreak _values :!label _label)
    (:LoopBody
      (if (== _array_element Actor)
        (Utilities|Map|Remove _debugactormap (.Key (Utilities|Map|GetKeyValueByIndex _debugactormap _array_index)))
        (goto _label Break)))
    (:Completed
      (Actor|DestroyActor Actor))))

(event Custom|SpawnHitTraceDebug
  (params (Hit :type Hit%20Result%20Structure) (TraceColour :type Linear%20Color%20Structure :default "(R=2.000000,G=0.000000,B=0.000000,A=1.000000)") (HitColour :type Linear%20Color%20Structure :default "(R=0.184238,G=2.000000,B=0.000000,A=1.000000)") (ArrowThickness :type Float%20%28single-precision%29) (DebugLifetime :type Float%20%28single-precision%29))
  (bind _returnvalue (Game|SpawnActorfromClass "/Game/Blueprints/Debug/BP_HitDebug.BP_HitDebug_C" (Transformation|GetActorTransform (Components|GetOwner)) "Undefined" "MultiplyWithRoot" 0 0))
  (Default|SpawnHit _returnvalue Hit TraceColour HitColour ArrowThickness)
  (Actor|SetLifeSpan _returnvalue DebugLifetime))
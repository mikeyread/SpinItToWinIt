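; Debug actor that draws spheres as mesh instances with a given colour, line width, location and size.
; BeginPlay creates a shared dynamic material and adds a first sphere; each SpawnDebugSpere call updates that material and adds a randomly rotated instance.
; Reaching the maximum count removes the oldest instance.
; A retriggerable delay clears all spheres after the last spawn's lifetime, then CallNoActiveSpheres signals that none remain.
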(event Custom|SpawnDebugSpere
  (params (SphereColour :type Linear%20Color%20Structure) (LineWidth :type Float%20%28single-precision%29) (Sphere%20Location :type Vector) (SpereSize :type Vector) (World%20Space :type Boolean) (MaxDebugSpheres :type Integer) (DebugLifeTime :type Float%20%28single-precision%29))
  (bind _debugsphere (Variables|Default|GetDebugSphere))
  (|SetVars SphereColour LineWidth Sphere%20Location SpereSize World%20Space MaxDebugSpheres DebugLifeTime)
  (Rendering|Material|SetVectorParameterValue (stale EventBeginPlay _output_get) "Colour" (Variables|Default|GetSphereColour) :!class /Script/Engine.MaterialInstanceDynamic)
  (Rendering|Material|SetScalarParameterValue (stale EventBeginPlay _output_get) "LineThickness" (Variables|Default|GetLineWidth) :!class /Script/Engine.MaterialInstanceDynamic)
  (bind _returnvalue (Components|InstancedStaticMesh|AddInstance _debugsphere (Math|Transform|MakeTransform (Variables|Default|GetSphere%20Location) (Math|Random|RandomRotator false) (Variables|Default|GetSpereSize)) (Variables|Default|GetWorld%20Space)))
  (if (>= _returnvalue (Variables|Default|GetMaxDebugSpheres))
    (Class|InstancedStaticMeshComponent|RemoveInstance _debugsphere)
    (if (== (Components|InstancedStaticMesh|GetInstanceCount _debugsphere) 0)
      _
      (else
        (Utilities|FlowControl|RetriggerableDelay (Variables|Default|GetDebugLifeTime) :!label _label)
        (Components|InstancedStaticMesh|ClearInstances _debugsphere)))
    (else
      (goto _label)))
  (Default|CallNoActiveSpheres self))

(event EventBeginPlay
  (bind _debugsphere (Variables|Default|GetDebugSphere))
  (bind _returnvalue (Rendering|Material|CreateDynamicMaterialInstance "/Game/Blueprints/Debug/M_DebugSphere.M_DebugSphere" "None" "None" :!class /Script/Engine.KismetMaterialLibrary))
  (bind _output_get (Variables|Default|SetSphereMaterial _returnvalue))
  (Rendering|Material|SetMaterial (Variables|Default|GetDebugSphere) 0 _output_get)
  (Rendering|Material|SetVectorParameterValue _output_get "Colour" (Variables|Default|GetSphereColour) :!class /Script/Engine.MaterialInstanceDynamic)
  (Rendering|Material|SetScalarParameterValue _output_get "LineThickness" (Variables|Default|GetLineWidth) :!class /Script/Engine.MaterialInstanceDynamic)
  (bind _returnvalue_2 (Components|InstancedStaticMesh|AddInstance _debugsphere (Math|Transform|MakeTransform (Variables|Default|GetSphere%20Location) (Math|Random|RandomRotator false) (Variables|Default|GetSpereSize)) (Variables|Default|GetWorld%20Space)))
  (if (>= _returnvalue_2 (Variables|Default|GetMaxDebugSpheres))
    (Class|InstancedStaticMeshComponent|RemoveInstance _debugsphere)
    (if (== (Components|InstancedStaticMesh|GetInstanceCount _debugsphere) 0)
      _
      (else
        (Utilities|FlowControl|RetriggerableDelay (Variables|Default|GetDebugLifeTime) :!label _label)
        (Components|InstancedStaticMesh|ClearInstances _debugsphere)))
    (else
      (goto _label)))
  (Default|CallNoActiveSpheres self))

(fn ConstructionScript)
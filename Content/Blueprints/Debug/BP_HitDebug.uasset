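; Debug actor that visualises a trace hit result with two arrow components, using colours and thickness passed to SpawnHit.
; On a blocking hit, TraceArrow spans trace start to impact point and HitArrow continues from impact to trace end.
; Without a hit, TraceArrow covers the whole trace and HitArrow is hidden.
; SpawnArrow positions, aims, colours and sizes each existing arrow, setting its length to the distance between endpoints.
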(event Custom|SpawnHit
  (params (Hit :type Hit%20Result%20Structure) (TraceColour :type Linear%20Color%20Structure :default "(R=0.184238,G=2.000000,B=0.000000,A=1.000000)") (HitColour :type Linear%20Color%20Structure :default "(R=2.000000,G=0.000000,B=0.000000,A=1.000000)") (ArrowThickness :type Float%20%28single-precision%29))
  (Variables|Default|SetHit Hit)
  (Variables|Default|SetTrace%20Colour TraceColour)
  (Variables|Default|SetHit%20Colour HitColour)
  (Variables|Default|SetArrow%20Thickness ArrowThickness)
  (if (.bBlockingHit (Collision|BreakHitResult (Variables|Default|GetHit)))
    (Utilities|FlowControl|Sequence
      (:then_0
        (CallFunction|SpawnArrow (Variables|Default|GetTraceArrow) (.TraceStart (Collision|BreakHitResult (Variables|Default|GetHit))) (.ImpactPoint (Collision|BreakHitResult (Variables|Default|GetHit))) (Variables|Default|GetTrace%20Colour) (Variables|Default|GetArrow%20Thickness)))
      (:then_1
        (CallFunction|SpawnArrow (Variables|Default|GetHitArrow) (.ImpactPoint (Collision|BreakHitResult (Variables|Default|GetHit))) (.TraceEnd (Collision|BreakHitResult (Variables|Default|GetHit))) (Variables|Default|GetHit%20Colour) (Variables|Default|GetArrow%20Thickness))))
    (else
      (CallFunction|SpawnArrow (Variables|Default|GetTraceArrow) (.TraceStart (Collision|BreakHitResult (Variables|Default|GetHit))) (.TraceEnd (Collision|BreakHitResult (Variables|Default|GetHit))) (Variables|Default|GetTrace%20Colour) (Variables|Default|GetArrow%20Thickness))
      (Development|SetHiddeninGame (Variables|Default|GetHitArrow) true false))))

(fn ConstructionScript)

(fn SpawnArrow
  (params (Arrow :type Arrow%20Component%20Object%20Reference) (ArrowStart :type Vector) (ArrowEnd :type Vector :default "0.000000,0.000000,1000.000000") (ArrowColour :type Linear%20Color%20Structure :default "(R=1.000000,G=0.000000,B=0.798977,A=1.000000)") (ArrowThickness :type Float%20%28single-precision%29))
  (Transformation|SetWorldLocationAndRotation Arrow ArrowStart (Math|Rotator|FindLookatRotation ArrowStart ArrowEnd) false false)
  (Components|Arrow|SetArrowColor(LinearColor) Arrow ArrowColour)
  (Variables|/Script/Engine.ArrowComponent|SetArrowSize Arrow ArrowThickness)
  (Variables|/Script/Engine.ArrowComponent|SetArrowLength Arrow (Math|Vector|Distance(Vector) ArrowStart ArrowEnd)))
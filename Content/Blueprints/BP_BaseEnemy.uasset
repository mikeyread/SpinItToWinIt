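; BP_BaseEnemy is an enemy that travels along a tagged BP_SplinePath at a randomized offset and can damage BP_Human at the path's end.
; A timeline scaled by TimeToComplete drives position and rotation along the spline, with events to stop and resume it.
; If DamageHuman is set, finishing damages the human's health component and destroys the enemy.
; Taking damage animates a dynamic overlay material on the visible Ant or Bee component as a hit flash.
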(event Custom|Move%20object
  (bind _human (Variables|Default|GetHuman))
  (bind _splinetrack (Variables|Default|GetSplineTrack))
  (bind _spline (Variables|/Game/Blueprints/BP_SplinePath.BP_SplinePath_C|GetSpline _splinetrack))
  (Components|Timeline|SetPlayRate (Variables|Default|GetT_Move) (/ 1.0 (Variables|Default|GetTimeToComplete)))
  (bind _move_track (Timeline|T_Move PlayFromStart)
    (:Update
      (Components|Timeline|SetPlayRate (Variables|Default|GetT_Move) (/ 1.0 (Variables|Default|GetTimeToComplete)))
      (Transformation|SetActorLocationAndRotation (+ (Spline|GetLocationatDistanceAlongSpline _spline (Math|Float|Lerp 0.0 (Spline|GetSplineLength _spline) _move_track) "World") (Variables|Default|GetSplineOffset)) (Spline|GetRotationatDistanceAlongSpline _spline (Math|Float|Lerp 0.0 (Spline|GetSplineLength _spline) _move_track) "World")))
    (:Finished
      (if (Variables|Default|GetDamageHuman)
        (Utilities|IsValid _human
          (:Is%20Valid
            (Default|TakeDamage (Variables|/Game/Blueprints/BP_Human.BP_Human_C|GetBPC_Health _human) (Variables|Default|GetDamageToHuman) "NewEnumerator0")
            (Actor|DestroyActor)))))))

(event Custom|Stop
  (bind _human (Variables|Default|GetHuman))
  (bind _splinetrack (Variables|Default|GetSplineTrack))
  (bind _spline (Variables|/Game/Blueprints/BP_SplinePath.BP_SplinePath_C|GetSpline _splinetrack))
  (Development|PrintString "stop")
  (bind _move_track (Timeline|T_Move Stop)
    (:Update
      (Components|Timeline|SetPlayRate (Variables|Default|GetT_Move) (/ 1.0 (Variables|Default|GetTimeToComplete)))
      (Transformation|SetActorLocationAndRotation (+ (Spline|GetLocationatDistanceAlongSpline _spline (Math|Float|Lerp 0.0 (Spline|GetSplineLength _spline) _move_track) "World") (Variables|Default|GetSplineOffset)) (Spline|GetRotationatDistanceAlongSpline _spline (Math|Float|Lerp 0.0 (Spline|GetSplineLength _spline) _move_track) "World")))
    (:Finished
      (if (Variables|Default|GetDamageHuman)
        (Utilities|IsValid _human
          (:Is%20Valid
            (Default|TakeDamage (Variables|/Game/Blueprints/BP_Human.BP_Human_C|GetBPC_Health _human) (Variables|Default|GetDamageToHuman) "NewEnumerator0")
            (Actor|DestroyActor)))))))

(event Custom|Resume
  (bind _human (Variables|Default|GetHuman))
  (bind _splinetrack (Variables|Default|GetSplineTrack))
  (bind _spline (Variables|/Game/Blueprints/BP_SplinePath.BP_SplinePath_C|GetSpline _splinetrack))
  (bind _move_track (Timeline|T_Move Play)
    (:Update
      (Components|Timeline|SetPlayRate (Variables|Default|GetT_Move) (/ 1.0 (Variables|Default|GetTimeToComplete)))
      (Transformation|SetActorLocationAndRotation (+ (Spline|GetLocationatDistanceAlongSpline _spline (Math|Float|Lerp 0.0 (Spline|GetSplineLength _spline) _move_track) "World") (Variables|Default|GetSplineOffset)) (Spline|GetRotationatDistanceAlongSpline _spline (Math|Float|Lerp 0.0 (Spline|GetSplineLength _spline) _move_track) "World")))
    (:Finished
      (if (Variables|Default|GetDamageHuman)
        (Utilities|IsValid _human
          (:Is%20Valid
            (Default|TakeDamage (Variables|/Game/Blueprints/BP_Human.BP_Human_C|GetBPC_Health _human) (Variables|Default|GetDamageToHuman) "NewEnumerator0")
            (Actor|DestroyActor)))))))

(event EventBeginPlay
  (bind _ant (Variables|Default|GetAnt))
  (bind _bee (Variables|Default|GetBee))
  (bind _splineoffsetmin (Variables|Default|GetSplineOffsetMin))
  (bind _splineoffsetmax (Variables|Default|GetSplineOffsetMax))
  (Variables|Default|SetSplineOffset (Math|Vector|MakeVector (Math|Random|RandomFloatinRange (.x _splineoffsetmin) (.x _splineoffsetmax)) (Math|Random|RandomFloatinRange (.y _splineoffsetmin) (.y _splineoffsetmax)) (Math|Random|RandomFloatinRange (.z _splineoffsetmin) (.z _splineoffsetmax))))
  (bind _outactors (Actor|GetAllActorsOfClasswithTag "/Game/Blueprints/BP_SplinePath.BP_SplinePath_C" (Variables|Default|GetSplineTag)))
  (Variables|Default|SetSplineTrack (Utilities|Array|Get(acopy) _outactors))
  (bind _returnvalue (Actor|GetActorOfClass "/Game/Blueprints/BP_Human.BP_Human_C"))
  (Variables|Default|SetHuman _returnvalue)
  (bind _returnvalue_2 (Rendering|Material|CreateDynamicMaterialInstance "/Game/Art/M_EnemyHit.M_EnemyHit" "None" "None" :!class /Script/Engine.KismetMaterialLibrary))
  (bind _output_get (Variables|Default|SetHitOverlay _returnvalue_2))
  (Utilities|FlowControl|Sequence
    (:then_0
      (if (Rendering|IsVisible _ant)
        (Rendering|Material|SetOverlayMaterial _ant _output_get :!class /Script/Engine.MeshComponent)
        (Development|PrintString "ANT")))
    (:then_1
      (if (Rendering|IsVisible _bee)
        (Rendering|Material|SetOverlayMaterial _bee _output_get :!class /Script/Engine.MeshComponent)
        (Development|PrintString "BEE")))
    (:then_2
      (CallFunction|MoveObject))))

(event Game|Damage|EventAnyDamage
  (params (Damage :type Float%20%28single-precision%29) (DamageType :type Damage%20Type%20Object%20Reference) (InstigatedBy :type Controller%20Object%20Reference) (DamageCauser :type Actor%20Object%20Reference))
  (bind _newtrack_0 (Timeline|Timeline PlayFromStart)
    (:Update
      (Rendering|Material|SetScalarParameterValue (Variables|Default|GetHitOverlay) "Alpha" _newtrack_0 :!class /Script/Engine.MaterialInstanceDynamic))))

(fn ConstructionScript
  (Variables|Default|SetTimeToComplete (Variables|Default|GetBaseTimeToComplete)))
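; BP_EnemySpawner spawns Ant or Bee enemies, chosen by EnemyToSpawn, along with recurring path VFX.
; BeginPlay starts a looping timer for BP_PathVFX actors and launches a single wave.
; The wave increments its counter and runs a looping one-second timer that spawns enemies and sets their base completion time.
; A spawned-enemy count clears the wave timer at its limit, while the path VFX keep spawning.
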(event Custom|StartSpawning
  (CallFunction|SpawnWave))

(event Custom|SpawnWave
  (Math|Integer|IncrementInt (Variables|Default|GetWaveCounter)
    (:%20%20
      (bind _returnvalue (Utilities|Time|SetTimerbyEvent (delegate Custom|SpawnEnemy) 1.0 true))
      (Variables|Default|SetWaveTimer _returnvalue))))

(event Custom|SpawnEnemy
  (bind _returnvalue (Game|SpawnActorfromClass (Utilities|Select :Index (Variables|Default|GetEnemyToSpawn) :NewEnumerator0 "/Game/Blueprints/BP_Enemy_Ant.BP_Enemy_Ant_C" :NewEnumerator1 "/Game/Blueprints/BP_Enemy_Bee.BP_Enemy_Bee_C") (Math|Transform|MakeTransform "0, 0, 0" "0, 0, 0" "1.000000,1.000000,1.000000") "Undefined" "MultiplyWithRoot" 0 0))
  (bind _asbp_base_enemy (Utilities|Casting|CastToBP_BaseEnemy _returnvalue))
  (Variables|/Game/Blueprints/BP_BaseEnemy.BP_BaseEnemy_C|SetBaseTimeToComplete _asbp_base_enemy 6e+01)
  (bind _result (Math|Integer|IncrementInt (Variables|Default|GetEnemiesSpawned))
    (:%20%20
      (if (>= _result 10)
        (Utilities|Time|ClearandInvalidateTimerbyHandle (Variables|Default|GetWaveTimer))))))

(event Custom|SpawnPathVFX
  (Game|SpawnActorfromClass "/Game/Blueprints/BP_PathVFX.BP_PathVFX_C" (Math|Transform|MakeTransform "0, 0, 0" "0, 0, 0" "1.000000,1.000000,1.000000") "Undefined" "MultiplyWithRoot" 0 3e+01 "-200.000000,200.000000,100.000000" "200.000000,200.000000,400.000000" 0))

(event EventBeginPlay
  (Utilities|Time|SetTimerbyEvent (delegate Custom|SpawnPathVFX) 3.0 true)
  (CallFunction|StartSpawning))

(fn ConstructionScript)
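; BP_Human is a damageable human that shows visual hit feedback on its skeletal mesh.
; On BeginPlay it creates a dynamic instance of M_EnemyHit and sets it as the mesh's overlay material.
; Any damage restarts a timeline that drives the overlay's Alpha parameter and debug-prints current health from BPCHealth on every update.
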(event Game|Damage|EventAnyDamage
  (params (Damage :type Float%20%28single-precision%29) (DamageType :type Damage%20Type%20Object%20Reference) (InstigatedBy :type Controller%20Object%20Reference) (DamageCauser :type Actor%20Object%20Reference))
  (bind _newtrack_0 (Timeline|Timeline PlayFromStart)
    (:Update
      (Rendering|Material|SetScalarParameterValue (Variables|Default|GetHitOverlay) "Alpha" _newtrack_0 :!class /Script/Engine.MaterialInstanceDynamic)
      (Development|PrintString (Utilities|String|ToString(Float) (Variables|/Game/Blueprints/Components/BPC_Health.BPC_Health_C|GetCurrentHealth (Variables|Default|GetBPC_Health)))))))

(event EventBeginPlay
  (bind _returnvalue (Rendering|Material|CreateDynamicMaterialInstance "/Game/Art/M_EnemyHit.M_EnemyHit" "None" "None" :!class /Script/Engine.KismetMaterialLibrary))
  (bind _output_get (Variables|Default|SetHitOverlay _returnvalue))
  (Rendering|Material|SetOverlayMaterial (Variables|Default|GetSkeletalMesh) _output_get :!class /Script/Engine.MeshComponent))

(fn ConstructionScript)
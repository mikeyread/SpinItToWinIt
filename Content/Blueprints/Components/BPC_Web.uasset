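; Actor component that manages a web resource pool, tracked as CurrentWeb.
; Tick refills it at a constant per-second rate through AddWeb, which runs only below MaxWeb but clamps to a hardcoded 100 rather than MaxWeb.
; ReduceWeb spends an amount only when enough web is available and returns whether it succeeded.
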(event EventTick
  (params (DeltaSeconds :type Float%20%28single-precision%29))
  (CallFunction|AddWeb (* DeltaSeconds 1e+01)))

(fn AddWeb
  (params (Added%20Web :type Float%20%28double-precision%29))
  (if (< (Variables|Default|GetCurrentWeb) (Variables|Default|GetMaxWeb))
    (Variables|Default|SetCurrentWeb (Math|Float|Min(Float) (+ Added%20Web (Variables|Default|GetCurrentWeb)) 1e+02))
    (return)))

(fn ReduceWeb
  (params (Amount :type Float%20%28double-precision%29))
  (if (>= (Variables|Default|GetCurrentWeb) Amount)
    (Variables|Default|SetCurrentWeb (Math|Float|Max(Float) (- (Variables|Default|GetCurrentWeb) Amount) 0.0))
    (return true)
    (else
      (return false))))
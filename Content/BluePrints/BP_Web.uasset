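; BP_Web is a web hazard that appears to slow enemies while they overlap its WebCollision.
; Begin overlap prints a debug string, casts to BP_BaseEnemy and sets its TimeToComplete to a large fixed value.
; End overlap restores BaseTimeToComplete, but only for the exact BP_BaseEnemy class, so subclasses keep the changed value.
; Disconnected leftover nodes hold a class check and Stop calls that never run.
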(event OnComponentBeginOverlap(WebCollision)
  (params (OverlappedComponent :type Primitive%20Component%20Object%20Reference) (OtherActor :type Actor%20Object%20Reference) (OtherComp :type Primitive%20Component%20Object%20Reference) (OtherBodyIndex :type Integer) (bFromSweep :type Boolean) (SweepResult :type Hit%20Result%20Structure%20%28by%20ref%29))
  (Development|PrintString "Hello")
  (bind _asbp_base_enemy (Utilities|Casting|CastToBP_BaseEnemy OtherActor))
  (Variables|/Game/Blueprints/BP_BaseEnemy.BP_BaseEnemy_C|SetTimeToComplete _asbp_base_enemy (Math|Float|MakeLiteralFloat 1e+03)))

(event OnComponentEndOverlap(WebCollision)
  (params (OverlappedComponent :type Primitive%20Component%20Object%20Reference) (OtherActor :type Actor%20Object%20Reference) (OtherComp :type Primitive%20Component%20Object%20Reference) (OtherBodyIndex :type Integer))
  (if (== (Utilities|GetClass OtherActor) "/Game/Blueprints/BP_BaseEnemy.BP_BaseEnemy_C")
    (bind _asbp_base_enemy (Utilities|Casting|CastToBP_BaseEnemy OtherActor))
    (Variables|/Game/Blueprints/BP_BaseEnemy.BP_BaseEnemy_C|SetTimeToComplete _asbp_base_enemy (Variables|/Game/Blueprints/BP_BaseEnemy.BP_BaseEnemy_C|GetBaseTimeToComplete _asbp_base_enemy))))

(fn ConstructionScript)
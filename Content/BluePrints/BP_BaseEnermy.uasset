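; BP_BaseEnermy is a base enemy actor that travels along the spline of a SplineTrack reference.
; The T_Move timeline maps its MoveTrack value to spline distance, setting world location and rotation, with play rate derived from TimeToComplete.
; Movement starts at BeginPlay, and Stop and Resume events halt and continue it.
; The construction script applies the configurable mesh and copies BaseTimeToComplete into TimeToComplete.
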(event Custom|Move%20object
  (bind _splinetrack (Variables|Default|GetSplineTrack))
  (bind _spline (Variables|/Game/BluePrints/BP_SplinePath.BP_SplinePath_C|GetSpline _splinetrack))
  (Components|Timeline|SetPlayRate (Variables|Default|GetT_Move) (/ 1.0 (Variables|Default|GetTimeToComplete)))
  (bind _move_track (Timeline|T_Move PlayFromStart)
    (:Update
      (Components|Timeline|SetPlayRate (Variables|Default|GetT_Move) (/ 1.0 (Variables|Default|GetTimeToComplete)))
      (Transformation|SetActorLocationAndRotation (Spline|GetLocationatDistanceAlongSpline _spline (Math|Float|Lerp 0.0 (Spline|GetSplineLength _spline) _move_track) "World") (Spline|GetRotationatDistanceAlongSpline _spline (Math|Float|Lerp 0.0 (Spline|GetSplineLength _spline) _move_track) "World")))))

(event Custom|Stop
  (bind _splinetrack (Variables|Default|GetSplineTrack))
  (bind _spline (Variables|/Game/BluePrints/BP_SplinePath.BP_SplinePath_C|GetSpline _splinetrack))
  (Development|PrintString "stop")
  (bind _move_track (Timeline|T_Move Stop)
    (:Update
      (Components|Timeline|SetPlayRate (Variables|Default|GetT_Move) (/ 1.0 (Variables|Default|GetTimeToComplete)))
      (Transformation|SetActorLocationAndRotation (Spline|GetLocationatDistanceAlongSpline _spline (Math|Float|Lerp 0.0 (Spline|GetSplineLength _spline) _move_track) "World") (Spline|GetRotationatDistanceAlongSpline _spline (Math|Float|Lerp 0.0 (Spline|GetSplineLength _spline) _move_track) "World")))))

(event Custom|Resume
  (bind _splinetrack (Variables|Default|GetSplineTrack))
  (bind _spline (Variables|/Game/BluePrints/BP_SplinePath.BP_SplinePath_C|GetSpline _splinetrack))
  (bind _move_track (Timeline|T_Move Play)
    (:Update
      (Components|Timeline|SetPlayRate (Variables|Default|GetT_Move) (/ 1.0 (Variables|Default|GetTimeToComplete)))
      (Transformation|SetActorLocationAndRotation (Spline|GetLocationatDistanceAlongSpline _spline (Math|Float|Lerp 0.0 (Spline|GetSplineLength _spline) _move_track) "World") (Spline|GetRotationatDistanceAlongSpline _spline (Math|Float|Lerp 0.0 (Spline|GetSplineLength _spline) _move_track) "World")))))

(event EventBeginPlay
  (CallFunction|MoveObject))

(event Collision|EventActorBeginOverlap
  (params (OtherActor :type Actor%20Object%20Reference)))

(event EventTick
  (params (DeltaSeconds :type Float%20%28single-precision%29)))

(fn ConstructionScript
  (Components|StaticMesh|SetStaticMesh (Variables|Default|GetStaticMesh) (Variables|Default|GetNew%20Mesh))
  (Variables|Default|SetTimeToComplete (Variables|Default|GetBaseTimeToComplete)))